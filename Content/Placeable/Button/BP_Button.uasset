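; BP_Button is a placeable interactable button that toggles a text indicator when used.
; On BeginPlay it colors ClickedText with its Color variable.
; Interact flips the Clicked flag, shows or hides the text to match and prints a debug message.
; EnableInteraction only prints the received flag, as its node for setting text visibility is disconnected.
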(event EventBeginPlay
  ;[1 1 1] Set Text Render Color to variable Color
  (Rendering|Components|TextRender|SetTextRenderColor (Variables|Default|GetClickedText) (Variables|Default|GetColor)))

(event Collision|EventActorBeginOverlap
  (params (OtherActor :type Actor%20Object%20Reference)))

(event EventTick
  (params (DeltaSeconds :type Float%20%28single-precision%29)))

(event EventEnableInteraction
  (params (Enable :type Boolean))
  ;[1 1 1] Set Visibility of Clicked Text to the value of "Enable" input
  (Development|PrintString (Utilities|String|Append "Enable Interaction: " (Utilities|String|ToString(Boolean) Enable))))

(event EventInteract
  (bind _output_get (Variables|Default|SetClicked (not (Variables|Default|GetClicked))))
  (Rendering|SetVisibility (Variables|Default|GetClickedText) _output_get false)
  (Development|PrintString "Clickado"))

(fn ConstructionScript)