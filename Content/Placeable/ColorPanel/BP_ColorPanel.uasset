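; Color panel actor that displays a color material on its screen, plays a matching sound, and shows current and high scores.
; Exposed events swap the screen material and sound, and play the audio for a given length using a delayed stop.
; On BeginPlay it finds BP_GameManager and binds to its round-won and game-over events.
; Won rounds update the score texts and high score, while game over resets the current score.
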(event Custom|GameLost
  ;[1 1 1] Reset Current Score and update CurrentScoreNumber text
  (bind _output_get (Variables|Default|SetCurrentScore 0))
  (CallFunction|AssignNumbertoTextRender _output_get (Variables|Default|GetCurrentScoreNumber)))

(event Custom|NextRound
  (params (RoundNumber :type Integer))
  ;[1 1 1] Assign Current Score to Current Score Number text
  (CallFunction|AssignNumbertoTextRender RoundNumber (Variables|Default|GetCurrentScoreNumber))
  ;[1 1 1] If Current Score is higher than High Score, update High Score and High Score Number text
  (if (> RoundNumber (Variables|Default|GetHighScore))
    (bind _output_get (Variables|Default|SetHighScore RoundNumber))
    (CallFunction|AssignNumbertoTextRender _output_get (Variables|Default|GetHighScoreNumber))))

(event EventBeginPlay
  ;[1 1 1] Find GameManager and add reference to variable
  (bind _returnvalue (Actor|GetActorOfClass "/Game/GameManager/BP_GameManager.BP_GameManager_C"))
  (bind _output_get (Variables|Default|SetGameManager _returnvalue))
  (EventDispatchers|BindEventtoRoundWon _output_get (delegate Custom|NextRound))
  (EventDispatchers|BindEventtoGameOver _output_get (delegate Custom|GameLost)))

(event EventSetColorSound
  (params (ColorSound :type Sound%20Wave%20Object%20Reference%20%28by%20ref%29))
  (Audio|Components|Audio|SetSound (Variables|Default|GetAudio) ColorSound))

(event EventSetMaterial
  (params (NewMaterial :type Material%20Instance%20Object%20Reference))
  (Rendering|Material|SetMaterial (Variables|Default|GetPanelColorScreen) 0 NewMaterial))

(event EventPlayColorSound
  (params (Length :type Float%20%28single-precision%29))
  (bind _output_get (Variables|Default|SetColorSoundLength Length))
  (bind (_shouldstopdelayed _playingtime) (CallFunction|PlaySoundfromAudio 0.0 _output_get (Variables|Default|GetColorSoundVolume)))
  (if _shouldstopdelayed
    (Utilities|FlowControl|Delay _playingtime)
    (Audio|Components|Audio|Stop (Variables|Default|GetAudio))))

(fn ConstructionScript)

(fn PlaySoundfromAudio
  (params (StartTime :type Float%20%28single-precision%29) (EndTime :type Float%20%28single-precision%29) (Volume :type Float%20%28single-precision%29))
  (bind _returnvalue (- EndTime StartTime))
  (bind _audio (Variables|Default|GetAudio))
  ;[1 1 1] Set volume multiplier in Audio component, and begin play
  (Audio|Components|Audio|SetVolumeMultiplier _audio Volume :!class /Script/Engine.AudioComponent)
  (Audio|Components|Audio|Play _audio StartTime)
  (return (> _returnvalue 0.0) _returnvalue))

(fn AssignNumbertoTextRender
  (params (Number :type Integer) (TextRender :type Text%20Render%20Component%20Object%20Reference%20%28by%20ref%29))
  (Rendering|Components|TextRender|SetText TextRender (Utilities|Text|ToText(Integer) Number)))