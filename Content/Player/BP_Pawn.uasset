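; VR player pawn that sets floor-level tracking and handles locomotion and hand interaction with actors.
; Controller colliders track BI_Interact actors with InteractableButton-tagged components per hand; Tick fires one interaction with haptics per trigger press.
; Tick also drives fixed-distance directional teleport steps from combined axis input, gated by deadzone and DoOnce.
; Axis events handle camera-compensated snap rotation and vertical movement input.
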(event OnComponentBeginOverlap(MotionControllerLeftCollider)
  (params (OverlappedComponent :type Primitive%20Component%20Object%20Reference) (OtherActor :type Actor%20Object%20Reference) (OtherComp :type Primitive%20Component%20Object%20Reference) (OtherBodyIndex :type Integer) (bFromSweep :type Boolean) (SweepResult :type Hit%20Result%20Structure%20%28by%20ref%29))
  ;[1 1 1] Enable Interaction with Actor whenever Controller Collider starts overlap (left/right)
  (CallFunction|EnableInteractionwhenCollidingComponentLeft OtherActor OtherComp))

(event OnComponentBeginOverlap(MotionControllerRightCollider)
  (params (OverlappedComponent :type Primitive%20Component%20Object%20Reference) (OtherActor :type Actor%20Object%20Reference) (OtherComp :type Primitive%20Component%20Object%20Reference) (OtherBodyIndex :type Integer) (bFromSweep :type Boolean) (SweepResult :type Hit%20Result%20Structure%20%28by%20ref%29))
  ;[1 1 1] Enable Interaction with Actor whenever Controller Collider starts overlap (left/right)
  (CallFunction|EnableInteractionwhenCollidingComponentRight OtherActor OtherComp))

(event OnComponentEndOverlap(MotionControllerLeftCollider)
  (params (OverlappedComponent :type Primitive%20Component%20Object%20Reference) (OtherActor :type Actor%20Object%20Reference) (OtherComp :type Primitive%20Component%20Object%20Reference) (OtherBodyIndex :type Integer))
  ;[1 1 1] Disable Interaction with Actor whenever Controller Collider finishes overlap (left/right)
  (CallFunction|DisableInteractionwhenCollidingComponentLeft OtherActor OtherComp))

(event OnComponentEndOverlap(MotionControllerRightCollider)
  (params (OverlappedComponent :type Primitive%20Component%20Object%20Reference) (OtherActor :type Actor%20Object%20Reference) (OtherComp :type Primitive%20Component%20Object%20Reference) (OtherBodyIndex :type Integer))
  ;[1 1 1] Disable Interaction with Actor whenever Controller Collider finishes overlap (left/right)
  (CallFunction|DisableInteractionwhenCollidingComponentRight OtherActor OtherComp))

(event EventBeginPlay
  ;[1 1 1] Set Tracking Origin to Floor at start of play
  (if (Class|HeadMountedDisplayFunctionLibrary|IsHeadMountedDisplayEnabled)
    (Class|HeadMountedDisplayFunctionLibrary|SetTrackingOrigin "Floor")))

(event Collision|EventActorBeginOverlap
  (params (OtherActor :type Actor%20Object%20Reference)))

(event EventTick
  (params (DeltaSeconds :type Float%20%28single-precision%29))
  (bind _returnvalue (Utilities|GetCombinedAxisMovement))
  ;[1 1 1] If pressing the left trigger & the InteractableActor for the left side is valid, interact with it and play haptic effect
  (if (Variables|Default|GetPressedTriggerLeft)
    (if (Variables|Default|GetIsInteractingLeft)
      _
      (else
        (bind _interactableactorleft (Variables|Default|GetInteractableActorLeft)
          (:then
            (Class|BIInteract|Interact(Message) _interactableactorleft)
            (Variables|Default|SetIsInteractingLeft true)
            (Utilities|PlayHapticVibrationLeft))
          (:else))))
    (else
      (Variables|Default|SetIsInteractingLeft false)))
  ;[1 1 1] If pressing the left trigger & the InteractableActor for the right side is valid, interact with it and play haptic effect
  (if (Variables|Default|GetPressedTriggerRight)
    (if (Variables|Default|GetIsInteractingRight)
      _
      (else
        (bind _interactableactorright (Variables|Default|GetInteractableActorRight)
          (:then
            (Class|BIInteract|Interact(Message) _interactableactorright)
            (Variables|Default|SetIsInteractingRight true)
            (Utilities|PlayHapticVibrationRight))
          (:else))))
    (else
      (Variables|Default|SetIsInteractingRight false)))
  ;[1 1 1] If combined axis magnitude > deadzone, teleport in the direction selected with the inputs
  (if (CallFunction|IsVectorMagnitudeOverThreshold _returnvalue)
    (Utilities|FlowControl|DoOnce false :!label _label
      (:Completed
        (CallFunction|TeleportMovement _returnvalue)))
    (else
      (goto _label Reset))))

(event Input|ActionEvents|InputActionTrigger_Left
  (params (Key :type Key%20Structure :default "None"))
  ;[1 1 1] Update "Pressed Trigger Left/Right" variable accordingly
  (:Pressed
    (Variables|Default|SetPressedTriggerLeft true))
  (:Released
    (Variables|Default|SetPressedTriggerLeft false)))

(event Input|ActionEvents|InputActionTrigger_Right
  (params (Key :type Key%20Structure :default "None"))
  ;[1 1 1] Update "Pressed Trigger Left/Right" variable accordingly
  (:Pressed
    (Variables|Default|SetPressedTriggerRight true))
  (:Released
    (Variables|Default|SetPressedTriggerRight false)))

(event Input|AxisEvents|InputAxisMovement_Z_Axis
  (params (AxisValue :type Float%20%28single-precision%29))
  ;[1 1 1] Move Pawn Up/Down
  (Pawn|Input|AddMovementInput (Math|Vector|GetUpVector (Variables|Default|GetDefaultSceneRoot)) (* AxisValue (Variables|Default|GetTeleportDistance)) false))

(event Input|AxisEvents|InputAxisMovement_X_Axis_Left
  (params (AxisValue :type Float%20%28single-precision%29))
  (bind _returnvalue (Transformation|GetActorLocation))
  (bind _returnvalue_2 (Math|Float|Round AxisValue))
  (bind _camera (Variables|Default|GetCamera))
  (bind _snaprotationdegrees (Variables|Default|GetSnapRotationDegrees))
  (bind _returnvalue_3 (* _returnvalue_2 _snaprotationdegrees))
  ;[1 1 1] Rotate Actor (adjusted to take into account camera transform)
  (if (CallFunction|IsAxisValueOverThreshold AxisValue)
    (Utilities|FlowControl|DoOnce false :!label _label
      (:Completed
        (Class|Actor|AddActorWorldRotation (Math|Rotator|MakeRotator 0.0 0.0 _returnvalue_3))
        (Transformation|SetActorLocation (+ (- (Transformation|GetWorldLocation _camera) (.location (Math|Transform|ComposeTransforms (Transformation|GetRelativeTransform _camera) (Math|Transform|MakeTransform _returnvalue (Math|Rotator|CombineRotators (Transformation|GetActorRotation) (Math|Rotator|MakeRotator 0.0 0.0 _returnvalue_3)))))) _returnvalue) false false)))
    (else
      (goto _label Reset))))

(fn ConstructionScript)

(fn EnableInteractionwhenCollidingComponentLeft
  (params (CollidingActor :type Actor%20Object%20Reference) (CollidingComponent :type Actor%20Component%20Object%20Reference))
  (if (and (Utilities|DoesObjectImplementInterface CollidingActor "/Game/Placeable/Interfaces/BI_Interact.BI_Interact_C") (Components|ComponentHasTag CollidingComponent "InteractableButton"))
    (bind _interactableactorleft (Variables|Default|GetInteractableActorLeft)
      (:then
        (if (not (== CollidingActor _interactableactorleft))
          (Class|BIInteract|EnableInteraction(Message) _interactableactorleft false)
          (bind _output_get (Variables|Default|SetInteractableActorLeft CollidingActor :!label _label))
          (Class|BIInteract|EnableInteraction(Message) _output_get true)))
      (:else
        (goto _label)))))

(fn EnableInteractionwhenCollidingComponentRight
  (params (CollidingActor :type Actor%20Object%20Reference) (CollidingComponent :type Actor%20Component%20Object%20Reference))
  (if (and (Utilities|DoesObjectImplementInterface CollidingActor "/Game/Placeable/Interfaces/BI_Interact.BI_Interact_C") (Components|ComponentHasTag CollidingComponent "InteractableButton"))
    (bind _interactableactorright (Variables|Default|GetInteractableActorRight)
      (:then
        (if (not (== CollidingActor _interactableactorright))
          (Class|BIInteract|EnableInteraction(Message) _interactableactorright false)
          (bind _output_get (Variables|Default|SetInteractableActorRight CollidingActor :!label _label))
          (Class|BIInteract|EnableInteraction(Message) _output_get true)))
      (:else
        (goto _label)))))

(fn DisableInteractionwhenCollidingComponentLeft
  (params (CollidingActor :type Actor%20Object%20Reference) (CollidingComponent :type Actor%20Component%20Object%20Reference))
  (if (and (Utilities|DoesObjectImplementInterface CollidingActor "/Game/Placeable/Interfaces/BI_Interact.BI_Interact_C") (Components|ComponentHasTag CollidingComponent "InteractableButton"))
    (if (Variables|Default|GetInteractableActorsMatchAtEndOverlap)
      (Class|BIInteract|EnableInteraction(Message) (stale _interactableactorright) false :!label _label)
      (Variables|Default|SetInteractableActorLeft 0 :!label _label_2)
      (else
        (bind _interactableactorright (Variables|Default|GetInteractableActorRight)
          (:then
            (if (== CollidingActor _interactableactorright)
              (Variables|Default|SetInteractableActorsMatchAtEndOverlap true)
              (else
                (goto _label))))
          (:else
            (goto _label_2)))))))

(fn DisableInteractionwhenCollidingComponentRight
  (params (CollidingActor :type Actor%20Object%20Reference) (CollidingComponent :type Actor%20Component%20Object%20Reference))
  (if (and (Utilities|DoesObjectImplementInterface CollidingActor "/Game/Placeable/Interfaces/BI_Interact.BI_Interact_C") (Components|ComponentHasTag CollidingComponent "InteractableButton"))
    (if (Variables|Default|GetInteractableActorsMatchAtEndOverlap)
      (Class|BIInteract|EnableInteraction(Message) (stale _interactableactorleft) false :!label _label)
      (Variables|Default|SetInteractableActorRight 0 :!label _label_2)
      (else
        (bind _interactableactorleft (Variables|Default|GetInteractableActorLeft)
          (:then
            (if (== CollidingActor _interactableactorleft)
              (Variables|Default|SetInteractableActorsMatchAtEndOverlap true)
              (else
                (goto _label))))
          (:else
            (goto _label_2)))))))

(fn IsAxisValueOverThreshold
  (params (AxisValue :type Float%20%28single-precision%29))
  (return (>= (Math|Float|Absolute(Float) AxisValue) (Variables|Default|GetAxisDeadzoneThreshold))))

(fn IsVectorMagnitudeOverThreshold
  (params (A :type Vector))
  (return (>= (Math|Vector|VectorLength A) (Variables|Default|GetAxisDeadzoneThreshold))))

(fn TeleportMovement
  (params (CombinedAxis :type Vector))
  (bind _returnvalue (Transformation|GetActorRotation))
  (bind _returnvalue_2 (Transformation|Teleport (+ (Transformation|GetWorldLocation (Variables|Default|GetDefaultSceneRoot)) (* (Math|Vector|RotateVector (Math|Vector|Normalize CombinedAxis (Variables|Default|GetAxisDeadzoneThreshold)) (Math|Rotator|MakeRotator 0.0 0.0 (.Yaw (Math|Rotator|BreakRotator _returnvalue)))) (Variables|Default|GetTeleportDistance))) _returnvalue))
  (return _returnvalue_2))