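; Game manager for a Simon-style memory game where players repeat a growing color sequence by clicking buttons.
; BeginPlay maps tagged buttons to color types, assigning materials and sounds.
; Each round appends a random color and replays the sequence on the color panel, with display time shrinking as score rises.
; Clicks are checked by tag, firing start, round-won or game-over dispatchers; button sound completion triggers the next round or reset.
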(event Custom|ResetGame
  ;[1 1 1] Set High Score to Current Score, and reset Current Score and Color Sequence
  (Variables|Default|SetHighScore (Variables|Default|GetCurrentScore))
  (Variables|Default|SetCurrentScore 0)
  (Utilities|Array|Clear (Variables|Default|GetColorSequence))
  ;[1 1 1] Listen to button clicks and reset End of Round bool
  (Variables|Default|SetListeningToButtonClicked true)
  (Variables|Default|SetEndOfRound false))

(event Custom|NextRound
  (bind _colorpanel (Variables|Default|GetColorPanel))
  (Variables|Default|SetShownColorTime (Math|Float|Lerp (Variables|Default|GetMaxShownColorTime) (Variables|Default|GetMinShownColorTime) (Math|Float|Min(Float) (/ (Math|Conversions|ToFloat(Integer) (Variables|Default|GetCurrentScore)) (Math|Conversions|ToFloat(Integer) (Variables|Default|GetFinalDifficultyRound))) 1.0)))
  ;[1 1 1] Reset Current Sequence Index and Current Round Color Sequence
  (Variables|Default|SetCurrentSequenceIndex 0)
  (Utilities|Array|Clear (Variables|Default|GetCurrentRoundColorSequence))
  ;[1 1 1] Get random ButtonType (except the Default type) and add to color sequence
  (Utilities|Array|Add (Variables|Default|GetColorSequence) (Utilities|Enum|ByteToEnumE_ButtonTypes (Math|Conversions|ToByte(Integer) (+ (Math|Random|RandomInteger (- (|GetNumEnumEntries) 1)) 1))))
  ;[1 1 1] For every element in Color Sequence, wait an instant before showing on Color Panel and play corresponding sound for a short time. Next, reset color and loop to next element
  (bind _arrayelement (Utilities|ForEachLoopforDelays (Variables|Default|GetColorSequence) :!label _label)
    (:LoopBody
      (Utilities|FlowControl|Delay (/ (Variables|Default|GetShownColorTime) 8.0))
      (Class|BISetMaterial|SetMaterial(Message) _colorpanel (.Value (Utilities|Map|Find (Variables|Default|GetButtonType_MaterialMap) _arrayelement)))
      (Class|BIColorSound|SetColorSound(Message) _colorpanel (.Value (Utilities|Map|Find (Variables|Default|GetButtonType_SoundMap) _arrayelement)))
      (Class|BIColorSound|PlayColorSound(Message) _colorpanel (Variables|Default|GetShownColorTime))
      (Utilities|FlowControl|Delay (Variables|Default|GetShownColorTime))
      (Class|BISetMaterial|SetMaterial(Message) (Variables|Default|GetColorPanel) (.Value (Utilities|Map|Find (Variables|Default|GetButtonType_MaterialMap) "NewEnumerator5")))
      (goto _label NextElement))
    (:Completed
      (Variables|Default|SetListeningToButtonClicked true)
      (Variables|Default|SetEndOfRound false)
      (Development|PrintString "Continue Game"))))

(event EventBeginPlay
  ;[1 1 1] Loop through all buttons
  (bind _outactors (Actor|GetAllActorsOfClass "/Game/Placeable/Button/BP_Button.BP_Button_C"))
  (for _array_element _outactors
    ;[1 1 1] If button has a button tag, add to ButtonType_ActorMap with the corresponding button type, set the correct material instance and sound and continue with the next button
    (Variables|Default|SetAddedTagToButton false)
    (bind _enumvalue (|ForEachE_ButtonTypes)
      (:LoopBody
        (if (Math|Boolean|ANDBoolean (Actor|ActorHasTag _array_element (.Value (Utilities|Map|Find (Variables|Default|GetButtonType_TagMap) _enumvalue))) (.ReturnValue (Utilities|Map|Find (Variables|Default|GetButtonType_TagMap) _enumvalue)) (not (Variables|Default|GetAddedTagToButton)))
          (Utilities|Map|Add (Variables|Default|GetButtonType_ActorMap) _enumvalue _array_element)
          (Variables|Default|SetAddedTagToButton true)
          (if (.ReturnValue (Utilities|Map|Find (Variables|Default|GetButtonType_MaterialMap) _enumvalue))
            (Class|BISetMaterial|SetMaterial(Message) _array_element (.Value (Utilities|Map|Find (Variables|Default|GetButtonType_MaterialMap) _enumvalue)))
            (Class|BIColorSound|SetColorSound(Message) _array_element (.Value (Utilities|Map|Find (Variables|Default|GetButtonType_SoundMap) _enumvalue))))))))
  ;[1 1 1] Find color panel actor, set to variable and set correct material instance
  (bind _returnvalue (Actor|GetActorOfClass "/Game/Placeable/ColorPanel/BP_ColorPanel.BP_ColorPanel_C"))
  (bind _output_get (Variables|Default|SetColorPanel _returnvalue))
  (Class|BISetMaterial|SetMaterial(Message) _output_get (.Value (Utilities|Map|Find (Variables|Default|GetButtonType_MaterialMap) "NewEnumerator5"))))

(event Collision|EventActorBeginOverlap
  (params (OtherActor :type Actor%20Object%20Reference)))

(event EventTick
  (params (DeltaSeconds :type Float%20%28single-precision%29)))

(event EventButtonClicked
  (params (ClickedButton :type BP%20Button%20Object%20Reference))
  (if (Variables|Default|GetListeningToButtonClicked)
    (Class|BIColorSound|PlayColorSound(Message) ClickedButton (Variables|Default|GetShownColorTime))
    ;[1 1 1] Check if the clicked Button is correct. (correct if button has the tag that matches with the current index in color in Current Round Color Sequence, incorrect otherwise). If incorrect, call Game Over and wait for button to finish playing Incorrect sound. If correct button, advance.
    (if (Utilities|Name|Equal(Name) (Utilities|Array|Get(acopy) (Variables|/Script/Engine.Actor|GetTags ClickedButton)) (.Value (Utilities|Map|Find (Variables|Default|GetButtonType_TagMap) (Utilities|Array|Get(acopy) (Variables|Default|GetColorSequence) (Variables|Default|GetCurrentSequenceIndex)))))
      ;[1 1 1] Check if game isn't active. If true, call Game Start, set game as active and wait for button to finish playing Correct sounds. Else, advance
      (if (not (Variables|Default|GetGameActive))
        (Default|CallGameStart)
        (bind _output_get (Variables|Default|SetGameActive true))
        (CallFunction|PlayandWaitforCorrectIncorrectButtonSound ClickedButton _output_get)
        (else
          ;[1 1 1] Add clicked color to Current Round Color Sequence. If its new size (last index + 1) matches Color Sequence size, increase Current Score, call Round Won dispatcher and wait for button to finish playing Correct sounds. Else, increment Current Sequence Index by one.
          (bind _returnvalue (Utilities|Array|Add (Variables|Default|GetCurrentRoundColorSequence) (Utilities|Array|Get(acopy) (Variables|Default|GetColorSequence) (Variables|Default|GetCurrentSequenceIndex))))
          (if (== (+ _returnvalue 1) (Utilities|Array|Length (Variables|Default|GetColorSequence)))
            (Utilities|IncreaseCurrentScore)
            (Default|CallRoundWon (Variables|Default|GetCurrentScore))
            (CallFunction|PlayandWaitforCorrectIncorrectButtonSound ClickedButton true)
            (else
              (Variables|Default|SetCurrentSequenceIndex (+ 1 (Variables|Default|GetCurrentSequenceIndex)))))))
      (else
        (bind _output_get_2 (Variables|Default|SetGameActive false))
        (Default|CallGameOver)
        (CallFunction|PlayandWaitforCorrectIncorrectButtonSound ClickedButton _output_get_2)))))

(event EventFinishedButtonCorrectIncorrectSound
  (if (Variables|Default|GetEndOfRound)
    (Utilities|FlowControl|Delay 0.5)
    (if (Variables|Default|GetGameActive)
      (CallFunction|NextRound)
      (else
        (CallFunction|ResetGame)))
    (else
      (Development|PrintString "Ignored Finished Button Correct Incoorect Sound: Not End of Round"))))

(fn ConstructionScript)

(fn WaitforFinishedButtonCorrectIncorrectSound
  (Variables|Default|SetEndOfRound true)
  (Variables|Default|SetListeningToButtonClicked false))

(fn PlayandWaitforCorrectIncorrectButtonSound
  (params (ButtonTarget :type Object%20Object%20Reference) (IsCorrect :type Boolean))
  (Class|BIColorSound|PlayCorrectIncorrectSound(Message) ButtonTarget IsCorrect)
  (CallFunction|WaitforFinishedButtonCorrectIncorrectSound))